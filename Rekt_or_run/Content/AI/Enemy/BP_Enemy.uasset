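; Enemy AI actor that turns perception of the player into blackboard state.
; Each tick it treats a leaning player as not visible, writes that flag, and ignores both sight and hearing updates while it is false.
; Sight and hearing handlers set seeing, hearing, lost-sight and last-known-location keys.
; Capsule contact with the player only prints a debug string, and flashlight detection is an empty stub.
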(event OnComponentHit(CapsuleComponent)
  (params (HitComponent :type Primitive%20Component%20Object%20Reference) (OtherActor :type Actor%20Object%20Reference) (OtherComp :type Primitive%20Component%20Object%20Reference) (NormalImpulse :type Vector :default "0, 0, 0") (Hit :type Hit%20Result%20Structure%20%28by%20ref%29))
  (if (== OtherActor (Game|GetPlayerCharacter 0))
    (Variables|Default|SetPlayerTouched true)
    (CallFunction|HandleTouchSensed)))

(event OnTargetPerceptionUpdated(Perception)
  (params (Actor :type Actor%20Object%20Reference) (Stimulus :type AI%20Stimulus%20Structure))
  (if (Variables|Default|GetisPlayerVisible)
    (CallFunction|HandleSightSensed Actor Stimulus)
    (CallFunction|HandleHearSensed Actor Stimulus)))

(event EventBeginPlay)

(event Collision|EventActorBeginOverlap
  (params (OtherActor :type Actor%20Object%20Reference)))

(event EventTick
  (params (DeltaSeconds :type Float%20%28single-precision%29))
  (bind _asbp_first_person_character (Utilities|Casting|CastToBP_FirstPersonCharacter (Game|GetPlayerCharacter 0)))
  (bind _output_get (Variables|Default|SetisPlayerVisible (not (Variables|/Game/FirstPerson/Blueprints/BP_FirstPersonCharacter.BP_FirstPersonCharacter_C|GetisLeaning _asbp_first_person_character))))
  (AI|Components|Blackboard|SetValueasBool (AI|GetBlackboard self) (Utilities|Name|MakeLiteralName "isPlayerVisible") _output_get))

(fn ConstructionScript)

(fn HandleSightSensed
  (params (Actor :type Actor%20Object%20Reference) (Stimulus :type AI%20Stimulus%20Structure))
  (bind _self self)
  (bind _returnvalue (AI|GetAIController _self))
  (bind _returnvalue_2 (AI|GetBlackboard _returnvalue))
  (bind _returnvalue_3 (Class|AIPerceptionSystem|GetSenseClassforStimulus Stimulus))
  (if (== _returnvalue_3 "/Script/AIModule.AISense_Sight")
    (if (.bsuccessfullysensed Stimulus)
      (AI|Components|Blackboard|SetValueasBool _returnvalue_2 (Utilities|Name|MakeLiteralName "isSeeingPlayer") true)
      (AI|Components|Blackboard|SetValueasBool _returnvalue_2 (Utilities|Name|MakeLiteralName "lostSight") false)
      (return)
      (else
        (AI|Components|Blackboard|SetValueasBool _returnvalue_2 (Utilities|Name|MakeLiteralName "isSeeingPlayer") false)
        (AI|Components|Blackboard|SetValueasVector _returnvalue_2 (Utilities|Name|MakeLiteralName "lastKnownLocation") (.stimuluslocation Stimulus))
        (AI|Components|Blackboard|SetValueasBool _returnvalue_2 (Utilities|Name|MakeLiteralName "lostSight") true)
        (return)))
    (else
      (return))))

(fn HandleHearSensed
  (params (actor :type Actor%20Object%20Reference) (stimulus :type AI%20Stimulus%20Structure))
  (bind _self self)
  (bind _returnvalue (AI|GetAIController _self))
  (bind _returnvalue_2 (AI|GetBlackboard _returnvalue))
  (bind _returnvalue_3 (Class|AIPerceptionSystem|GetSenseClassforStimulus stimulus))
  (if (== _returnvalue_3 "/Script/AIModule.AISense_Hearing")
    (if (.bsuccessfullysensed stimulus)
      (AI|Components|Blackboard|SetValueasBool _returnvalue_2 (Utilities|Name|MakeLiteralName "isHearingPlayer") (.bsuccessfullysensed stimulus))
      (AI|Components|Blackboard|SetValueasVector _returnvalue_2 (Utilities|Name|MakeLiteralName "lastKnownLocation") (.stimuluslocation stimulus))
      (return))
    (else
      (return))))

(fn HandleFlashlightSeen)

(fn HandleTouchSensed
  (params (actor :type Actor%20Object%20Reference) (stimuli :type AI%20Stimulus%20Structure))
  (if (Variables|Default|GetPlayerTouched)
    (Development|PrintString "TykTykTyk" true true "(R=1.000000,G=0.000000,B=0.893594,A=1.000000)")
    (Variables|Default|SetPlayerTouched false)
    (else
      (return))))