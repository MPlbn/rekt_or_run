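; Green door Blueprint that swings open or shut on Interact when the player character has the green key.
; Interact casts the player to BP_FirstPersonCharacter, checks HasGreenKey, then toggles IsOpening to play or reverse Door_Timeline.
; The timeline lerps the Door's relative yaw, while IsDuringOpening blocks input until it finishes.
; IsFinished is set during updates but is not read here.
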(event EventInteract
  (bind _asbp_first_person_character (Utilities|Casting|CastToBP_FirstPersonCharacter (Game|GetPlayerCharacter 0)))
  (if (Variables|/Game/FirstPerson/Blueprints/BP_FirstPersonCharacter.BP_FirstPersonCharacter_C|GethasGreenKey _asbp_first_person_character)
    (if (not (Variables|Default|GetisDuringOpening))
      (Variables|Default|SetisDuringOpening true)
      (bind _output_get (Variables|Default|SetisOpening (not (Variables|Default|GetisOpening))))
      (if _output_get
        (bind _door_alpha (Timeline|Door_Timeline Play)
          (:Update
            (Transformation|SetRelativeRotation (Variables|Actor|GetDoor) (Math|Rotator|MakeRotator 0.0 0.0 (Math|Float|Lerp 0.0 -1.1e+02 _door_alpha)) false false)
            ;[1 1 1] for later use maybe
            (Variables|Default|SetisFinished true))
          (:Finished
            (Variables|Default|SetisDuringOpening false)))
        (else
          (Timeline|Door_Timeline Reverse))))))

(fn ConstructionScript)