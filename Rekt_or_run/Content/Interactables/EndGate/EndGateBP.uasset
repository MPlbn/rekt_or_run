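; End gate interactable that finishes the game once the player has collected all notes.
; Interact checks HasAllNotes on the first-person character and opens MainMenuLevel when it is true.
; GiveInfo uses the same flag to pick either a pass-the-exam prompt or a collect-the-notes hint, then shows it through the HUD widget.
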(event EventGiveInfo
  (bind _asnew_hud (Utilities|Casting|CastToNewHUD (HUD|GetHUD (Game|GetPlayerController 0))))
  (bind _asbp_first_person_character (Utilities|Casting|CastToBP_FirstPersonCharacter (Game|GetPlayerCharacter 0)))
  (if (Variables|/Game/FirstPerson/Blueprints/BP_FirstPersonCharacter.BP_FirstPersonCharacter_C|GethasAllNotes _asbp_first_person_character)
    (Variables|Default|SetcurrentText "Press \"F\" to pass the exam")
    (else
      (Variables|Default|SetcurrentText "You need to collect all the notes!")))
  (Default|SetNewText (Variables|/Game/GUI/NewHUD.NewHUD_C|GetUI_ref _asnew_hud) (Variables|Default|GetcurrentText))
  (Default|ShowInfo (Variables|/Game/GUI/NewHUD.NewHUD_C|GetUI_ref _asnew_hud)))

(event EventInteract
  (bind _asbp_first_person_character (Utilities|Casting|CastToBP_FirstPersonCharacter (Game|GetPlayerCharacter 0)))
  (if (Variables|/Game/FirstPerson/Blueprints/BP_FirstPersonCharacter.BP_FirstPersonCharacter_C|GethasAllNotes _asbp_first_person_character)
    (Game|OpenLevel(byName) "MainMenuLevel")))

(fn ConstructionScript)