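; Readable note pickup that the first-person character can open and close while standing near it.
; A Box overlap tracks whether the player is close, and Interact only toggles reading while in range.
; Picking up creates a widget on the viewport, putting down removes it, and both play a page sound at the mesh.
; Walking out of the box automatically puts an open note down.
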(event OnComponentEndOverlap(Box)
  (params (OverlappedComponent :type Primitive%20Component%20Object%20Reference) (OtherActor :type Actor%20Object%20Reference) (OtherComp :type Primitive%20Component%20Object%20Reference) (OtherBodyIndex :type Integer))
  (Utilities|Casting|CastToBP_FirstPersonCharacter OtherActor)
  (Utilities|FlowControl|Sequence
    (:then_0
      (Variables|Default|SetisClose false)
      (if (Variables|Default|GetisReading)
        (CallFunction|PutDownNote)))))

(event OnComponentBeginOverlap(Box)
  (params (OverlappedComponent :type Primitive%20Component%20Object%20Reference) (OtherActor :type Actor%20Object%20Reference) (OtherComp :type Primitive%20Component%20Object%20Reference) (OtherBodyIndex :type Integer) (bFromSweep :type Boolean) (SweepResult :type Hit%20Result%20Structure%20%28by%20ref%29))
  (Utilities|Casting|CastToBP_FirstPersonCharacter OtherActor)
  (Variables|Default|SetisClose true))

(event Custom|PutDownNote
  (Audio|PlaySoundatLocation "/Game/Interactables/Notes/NoteMesh/pageSound.pageSound" (Transformation|GetWorldLocation (Variables|Default|GetStaticMesh)) "0, 0, 0" 1.0 1.0 0.0 0 0 0 0)
  (Widget|RemovefromParent (stale Custom|PickupNote _returnvalue))
  (Variables|Default|SetisReading false))

(event Custom|TogglePickUp
  (if (Variables|Default|GetisReading)
    (CallFunction|PutDownNote)
    (else
      (CallFunction|PickupNote))))

(event Custom|PickupNote
  (Audio|PlaySoundatLocation "/Game/Interactables/Notes/NoteMesh/pageSound.pageSound" (Transformation|GetWorldLocation (Variables|Default|GetStaticMesh)) "0, 0, 0" 1.0 1.0 0.0 0 0 0 0)
  (bind _returnvalue (UserInterface|CreateWidget (Variables|Default|GetClass)))
  (UserInterface|Viewport|AddtoViewport _returnvalue 0)
  (Variables|Default|SetisReading true))

(event EventInteract
  (if (Variables|Default|GetisClose)
    (CallFunction|TogglePickUp)))

(fn ConstructionScript)